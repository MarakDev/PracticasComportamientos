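; BP_SoldierAI is an AI controller that sends its soldier pawn wandering between BP_Waypoint actors.
; After a random delay, it gathers every unlocked waypoint whose AllowedAccess lists the controlled BP_AI_Character, shuffles them and moves to the first.
; The chosen waypoint stays locked during the move, reserving it from other selections.
; Move completion, whatever the result, unlocks it, clears the list and repeats the cycle after another random delay.
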(event Custom|ReciveMoveCompleted_Event
  (params (RequestID :type AI%20Request%20ID%20Structure) (Result :type EPathFollowingResult%20Enum :default "Success"))
  (bind _routes (Variables|Default|GetRoutes))
  (bind _routes_2 (Variables|Default|GetRoutes))
  (bind _output (Utilities|Array|Get(acopy) _routes_2))
  (Variables|/Game/Blueprints/BP_Waypoint.BP_Waypoint_C|SetLocked (Utilities|Array|Get(acopy) _routes) false)
  (Utilities|Array|Clear _routes)
  (Utilities|FlowControl|Delay (* (Math|Random|RandomFloat) 2.0))
  (bind _outactors (Actor|GetAllActorsOfClass "/Game/Blueprints/BP_Waypoint.BP_Waypoint_C"))
  (bind _asbp_ai_character (Utilities|Casting|CastToBP_AI_Character (Pawn|GetControlledPawn)))
  (for _array_element _outactors
    (if (not (Variables|/Game/Blueprints/BP_Waypoint.BP_Waypoint_C|GetLocked _array_element))
      (if (!= (Utilities|Array|FindItem (Variables|/Game/Blueprints/BP_Waypoint.BP_Waypoint_C|GetAllowedAccess _array_element) _asbp_ai_character) -1)
        (Utilities|Array|Add _routes_2 _array_element))))
  (Utilities|Array|Shuffle _routes_2)
  (Variables|/Game/Blueprints/BP_Waypoint.BP_Waypoint_C|SetLocked _output true)
  (AI|Navigation|MovetoActor _output -1.0 true true true 0))

(event EventBeginPlay
  (bind _routes (Variables|Default|GetRoutes))
  (bind _output (Utilities|Array|Get(acopy) _routes))
  (EventDispatchers|BindEventtoReceiveMoveCompleted (delegate Custom|ReciveMoveCompleted_Event))
  (Utilities|FlowControl|Delay (Math|Random|RandomFloat))
  (bind _outactors (Actor|GetAllActorsOfClass "/Game/Blueprints/BP_Waypoint.BP_Waypoint_C"))
  (bind _asbp_ai_character (Utilities|Casting|CastToBP_AI_Character (Pawn|GetControlledPawn)))
  (for _array_element _outactors
    (if (not (Variables|/Game/Blueprints/BP_Waypoint.BP_Waypoint_C|GetLocked _array_element))
      (if (!= (Utilities|Array|FindItem (Variables|/Game/Blueprints/BP_Waypoint.BP_Waypoint_C|GetAllowedAccess _array_element) _asbp_ai_character) -1)
        (Utilities|Array|Add _routes _array_element))))
  (Utilities|Array|Shuffle _routes)
  (Variables|/Game/Blueprints/BP_Waypoint.BP_Waypoint_C|SetLocked _output true)
  (AI|Navigation|MovetoActor _output -1.0 true true true 0))

(fn ConstructionScript)